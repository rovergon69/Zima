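; Krasny matrioska proxy actor that lets a nearby Zelty player character change into Krasny.
; The 2 key or MatrioskaChange input checks distance and idle state, calls ChangeToKrasny, turns toward the player and plays ReverseOpens_Anim.
; After a short delay, it spawns the Krasny character at the player's position and destroys itself.
; A separate checkOutHigh event fakes gravity with a downward trace and self-calling Delay loop.
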(event `self.ReceiveBeginPlay`
  ;[1 1 1] whatMakesEverythingWork
  (`self.EnableInput` (`GameplayStatics.GetPlayerController` 0)))

(event `Key|Two` :consume false
  (params (Key :type "Key Structure"))
  (bind (_transform_location _transform_rotation _transform_scale) (`KismetMathLibrary.BreakTransform` (`self.transform`)))
  (:`Pressed`
    ;[0.8605 0.2305 1] posible
    (if (< (`KismetMathLibrary.Vector_Distance` (`self.K2_GetActorLocation` (`GameplayStatics.GetPlayerCharacter` 0)) (`self.K2_GetActorLocation`)) 20.0) :!label _label
      (bind _asbp_third_person_character_matrioska_zelty (cast `/Game/matrioska/BP_ThirdPersonCharacterMatrioskaZelty` (`GameplayStatics.GetPlayerCharacter` 0)))
      (if (not (or (`/Game/matrioska/BP_ThirdPersonCharacterMatrioskaZelty.jumping` _asbp_third_person_character_matrioska_zelty) (`/Game/matrioska/BP_ThirdPersonCharacterMatrioskaZelty.attacking` _asbp_third_person_character_matrioska_zelty) (`/Game/matrioska/BP_ThirdPersonCharacterMatrioskaZelty.isChanging` _asbp_third_person_character_matrioska_zelty) (`NavMovementComponent.IsFalling` (`Character.CharacterMovement` _asbp_third_person_character_matrioska_zelty))))
        ;[0.1717 0.2 1] logic
        (`/Game/matrioska/BP_ThirdPersonCharacterMatrioskaZelty.changeToKrasny` _asbp_third_person_character_matrioska_zelty)
        (set `self.transform` (`self.GetTransform` (`GameplayStatics.GetPlayerCharacter` 0)))
        (set `self.rotation` (`self.K2_GetActorRotation`))
        (`self.K2_SetActorRotation` (`KismetMathLibrary.Conv_VectorToRotator` (* (- (`self.K2_GetActorLocation`) (`self.K2_GetActorLocation` (`GameplayStatics.GetPlayerCharacter` 0))) (-1.0 -1.0 0.0))))
        (`SkeletalMeshComponent.PlayAnimation` (`self.SkeletalMesh`) "/Game/matrioska/ChangeAnimation/reverseOpens_Anim.reverseOpens_Anim" false)
        (`PrimitiveComponent.SetCollisionEnabled` (`self.SkeletalMesh`) "NoCollision")
        ;[0.5427 1 0.4039] fireworks
        (`KismetSystemLibrary.Delay` 0.4)
        (set `self.rotation` (struct))
        (`|SpawnActorFromClass` "/Game/matrioska/BP_ThirdPersonCharacterMatrioskaKrasny.BP_ThirdPersonCharacterMatrioskaKrasny_C" (`KismetMathLibrary.MakeTransform` (+ _transform_location (0.0 0.0 5.0)) (struct) _transform_scale) "Undefined" "OverrideRootScale" null null)
        (`self.K2_DestroyActor`)))))

(event `InputAction|MatrioskaChange` :consume false
  (params (Key :type "Key Structure"))
  (:`Pressed`
    (goto _label)))

(event `checkOutHigh`
  (bind (_returnvalue_x _returnvalue_y _returnvalue_z) (`KismetMathLibrary.BreakVector` (`self.K2_GetActorLocation`)))
  (bind _skeletalmesh (`self.SkeletalMesh`))
  (bind _returnvalue (`SceneComponent.K2_GetComponentLocation` (`self.SkeletalMesh`)))
  (bind (_returnvalue_x_2 _returnvalue_y_2 _returnvalue_z_2) (`KismetMathLibrary.BreakVector` (`SceneComponent.K2_GetComponentLocation` _skeletalmesh)))
  ;[1 1 1] checkHigh
  (bind _outhit (`KismetSystemLibrary.LineTraceSingle` _returnvalue (- _returnvalue (0.0 0.0 1000.0)) "TraceTypeQuery1"))
  (bind (_bblockinghit _binitialoverlap _time _distance) (`GameplayStatics.BreakHitResult` _outhit))
  (if (> _distance 1.828949)
    (`self.K2_SetActorLocation` (`KismetMathLibrary.MakeVector` _returnvalue_x _returnvalue_y (- _returnvalue_z (`self.fallingSpeed`))))
    (`KismetSystemLibrary.Delay` 0.01)
    (set `self.fallingSpeed` (+ (`self.fallingSpeed`) 0.7))
    (`self.checkOutHigh`)
    (elif (> _distance 1.1)
      (set `self.fallingSpeed` 1.0)
      (else
        (`SceneComponent.K2_SetWorldLocation` _skeletalmesh (`KismetMathLibrary.MakeVector` _returnvalue_x_2 _returnvalue_y_2 (+ _returnvalue_z_2 2.0)) false false)
        (set `self.fallingSpeed` 1.0)))))

(fn `UserConstructionScript`)