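; Obstacle the player shoves with a left click while inside its Box trigger, provided the matrioska character's Strength covers its Weight.
; Strength comes from casting to the Krasny, Zelty or Siren character.
; After a short delay, the push follows the dominant X/Y offset away from the player, gated by CheckOrient's yaw-facing windows.
; Physics is enabled for an AddForce scaled by distance and strength, then disabled a second later.
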(event `self.Box.OnComponentBeginOverlap`
  (params (OverlappedComponent :type "PrimitiveComponent Object Reference") (OtherActor :type "Actor Object Reference") (OtherComp :type "PrimitiveComponent Object Reference") (OtherBodyIndex :type Integer) (bFromSweep :type Boolean) (SweepResult :type "HitResult Structure (by ref)"))
  ;[1 0.05313 0.05313] IsInRannge
  (if (== OtherActor (`GameplayStatics.GetPlayerCharacter` 0))
    (set `self.isInRaange` true)))

(event `self.ReceiveBeginPlay`
  ;[1 1 1] whatMakesEverythingWork
  (`self.EnableInput` (`GameplayStatics.GetPlayerController` 0)))

(event `self.Box.OnComponentEndOverlap`
  (params (OverlappedComponent :type "PrimitiveComponent Object Reference") (OtherActor :type "Actor Object Reference") (OtherComp :type "PrimitiveComponent Object Reference") (OtherBodyIndex :type Integer))
  ;[1 0.05313 0.05313] IsInRannge
  (if (== OtherActor (`GameplayStatics.GetPlayerCharacter` 0))
    (set `self.isInRaange` false)))

(event `Key|LeftMouseButton` :consume false
  (params (Key :type "Key Structure"))
  (bind (_x_ _x__2 _y_ _y__2) (`self.checkOrient`))
  (bind _returnvalue (`GameplayStatics.GetPlayerCharacter` 0))
  (bind _returnvalue_2 (* (* (`self.Strenght`) 100) (`self.extraStrenght`)))
  (bind (_returnvalue_x _returnvalue_y) (`KismetMathLibrary.BreakVector` (- (`SceneComponent.K2_GetComponentLocation` (`self.mesh`)) (`SceneComponent.K2_GetComponentLocation` (`Actor.RootComponent` (`GameplayStatics.GetPlayerCharacter` 0))))))
  (bind _returnvalue_3 (`KismetMathLibrary.Abs` _returnvalue_y))
  (bind _returnvalue_4 (`KismetMathLibrary.Abs` _returnvalue_x))
  (bind _returnvalue_5 (* _returnvalue_3 _returnvalue_2))
  (bind _returnvalue_6 (* _returnvalue_2 _returnvalue_4))
  ;[0 0.145 1] Pre
  (:`Pressed`
    (if (`self.isInRaange`)
      (bind _asbp_third_person_character_matrioska_krasny (cast `/Game/matrioska/BP_ThirdPersonCharacterMatrioskaKrasny` _returnvalue)
        (:`then`
          (set `self.Strenght` (`/Game/matrioska/BP_ThirdPersonCharacterMatrioskaKrasny.strength` _asbp_third_person_character_matrioska_krasny)))
        (:`CastFailed`
          (bind _asbp_third_person_character_matrioska_zelty (cast `/Game/matrioska/BP_ThirdPersonCharacterMatrioskaZelty` _returnvalue)
            (:`then`
              (set `self.Strenght` (`/Game/matrioska/BP_ThirdPersonCharacterMatrioskaZelty.strength` _asbp_third_person_character_matrioska_zelty)))
            (:`CastFailed`
              (bind _asbp_third_person_character_matrioska_siren (cast `/Game/matrioska/BP_ThirdPersonCharacterMatrioskaSiren` _returnvalue))
              (set `self.Strenght` (`/Game/matrioska/BP_ThirdPersonCharacterMatrioskaSiren.strength` _asbp_third_person_character_matrioska_siren))))))
      (`KismetSystemLibrary.Delay` 0.6)
      (if (`self.isInRaange`)
        (if (<= (`self.weight`) (`self.Strenght`))
          (`PrimitiveComponent.SetSimulatePhysics` (`self.mesh`) true)
          ;[1 0.638 0.01441] Calculus
          (if (< _returnvalue_4 _returnvalue_3)
            ;[1 1 1] strengthDirection
            (if (< _returnvalue_y 0.0)
              ;[0.7145 0 1] FaceOrnotToFace
              (if _x__2
                ;[0.4141 1 0.2102] Results
                (`PrimitiveComponent.AddForce` (`self.mesh`) (`KismetMathLibrary.MakeVector` 0.0 (* _returnvalue_5 -1.0)) "None" true)
                (`KismetSystemLibrary.Delay` 1.0 :!label _label)
                (`PrimitiveComponent.SetSimulatePhysics` (`self.mesh`) false))
              (elif _x_
                (`PrimitiveComponent.AddForce` (`self.mesh`) (`KismetMathLibrary.MakeVector` 0.0 _returnvalue_5) "None" true)
                (goto _label)))
            (elif (< _returnvalue_x 0.0)
              (if _y_
                (`PrimitiveComponent.AddForce` (`self.mesh`) (`KismetMathLibrary.MakeVector` (* _returnvalue_6 -1.0)) "None" true)
                (goto _label))
              (elif _y__2
                (`PrimitiveComponent.AddForce` (`self.mesh`) (`KismetMathLibrary.MakeVector` _returnvalue_6) "None" true)
                (goto _label)))))))))

(fn `checkOrient`
  (returns (`x+` :type Boolean) (`x-` :type Boolean) (`y+` :type Boolean) (`y-` :type Boolean))
  (bind (_returnvalue_roll _returnvalue_pitch _returnvalue_yaw) (`KismetMathLibrary.BreakRotator` (`SceneComponent.K2_GetComponentRotation` (`self.mesh`))))
  (bind (_returnvalue_roll_2 _returnvalue_pitch_2 _returnvalue_yaw_2) (`KismetMathLibrary.BreakRotator` (`SceneComponent.K2_GetComponentRotation` (`Actor.RootComponent` (`GameplayStatics.GetPlayerCharacter` 0)))))
  (bind _returnvalue (- _returnvalue_yaw_2 _returnvalue_yaw))
  (return (and (> _returnvalue 75.0) (< _returnvalue 105.0)) (or (and (> _returnvalue 255.0) (< _returnvalue 285.0)) (and (< _returnvalue -75.0) (> _returnvalue -105.0))) (or (and (> _returnvalue -195.0) (< _returnvalue -165.0)) (and (> _returnvalue 165.0) (< _returnvalue 195.0))) (and (> _returnvalue -15.0) (< _returnvalue 15.0))))

(fn `UserConstructionScript`)