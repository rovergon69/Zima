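; Follow-camera actor that trails player 0's pawn on X and Y while keeping its own height, with field of view set at construction.
; BeginPlay snaps X to the pawn, records its Y and starts a looping timer that replays the Value timeline.
; Timeline updates interpolate toward the pawn's X plus its Y movement delta at curve-scaled constant speed.
; If the pawn becomes invalid mid-update, it polls each tick before resuming.
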(event `self.ReceiveBeginPlay`
  (bind (_returnvalue_x _returnvalue_y _returnvalue_z) (`KismetMathLibrary.BreakVector` (`self.K2_GetActorLocation`)))
  (bind (_returnvalue_x_2 _returnvalue_y_2) (`KismetMathLibrary.BreakVector` (`self.K2_GetActorLocation` (`GameplayStatics.GetPlayerPawn` 0))))
  (bind _returnvalue_x_3 (`KismetMathLibrary.BreakVector` (`self.K2_GetActorLocation` (`GameplayStatics.GetPlayerPawn` 0))))
  ;[1 1 1] InitialValues
  (set `self.BaseY` _returnvalue_y_2)
  (`KismetSystemLibrary.K2_SetTimerDelegate` (delegate `Cam`) 1.5 true)
  (`self.K2_SetActorLocation` (`KismetMathLibrary.MakeVector` _returnvalue_x_3 _returnvalue_y _returnvalue_z) true true))

(event `Cam`
  (bind _returnvalue (`GameplayStatics.GetWorldDeltaSeconds`))
  (bind _returnvalue_2 (`GameplayStatics.GetPlayerPawn` 0))
  (bind (_returnvalue_x _returnvalue_y _returnvalue_z) (`KismetMathLibrary.BreakVector` (`self.K2_GetActorLocation`)))
  (bind _returnvalue_3 (`GameplayStatics.GetPlayerPawn` 0))
  (bind (_returnvalue_x_2 _returnvalue_y_2) (`KismetMathLibrary.BreakVector` (`self.K2_GetActorLocation` _returnvalue_2)))
  (bind (_returnvalue_x_3 _returnvalue_y_3) (`KismetMathLibrary.BreakVector` (`self.K2_GetActorLocation` (`GameplayStatics.GetPlayerPawn` 0))))
  ;[1 1 1] CamFollow
  (`/Engine/EditorBlueprintResources/StandardMacros.IsValid` _returnvalue_2
    (:`Is Valid`
      ;;[1 1 1] animate
      (bind (_direction _value) (`Timeline|value` :`NewTime` _returnvalue :!via `PlayFromStart` :!label _label)
        (:`Update`
          ;;[1 1 1] FixChange
          (`/Engine/EditorBlueprintResources/StandardMacros.IsValid` _returnvalue_3
            (:`Is Valid`
              ;;[1 1 1] valuesEnd
              (`self.K2_SetActorLocation` (`KismetMathLibrary.VInterpTo_Constant` (`self.K2_GetActorLocation`) (`KismetMathLibrary.MakeVector` _returnvalue_x_2 (+ (- _returnvalue_y_2 (`self.BaseY`)) _returnvalue_y) _returnvalue_z) _returnvalue (* _value (`self.valueOfFuse`))) true true)
              (set `self.BaseY` _returnvalue_y_3))
            (:`Is Not Valid`
              (`KismetSystemLibrary.DelayUntilNextTick` :!label _label_2)
              (`/Engine/EditorBlueprintResources/StandardMacros.IsValid` _returnvalue_3
                (:`Is Valid`
                  (goto _label))
                (:`Is Not Valid`
                  (goto _label_2))))))))))

(fn `UserConstructionScript`
  (`CameraComponent.SetFieldOfView` (`self.Camera`) (`self.Field Of View`)))