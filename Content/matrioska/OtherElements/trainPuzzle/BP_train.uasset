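; BP_train is a puzzle train that the player shunts between two positions with a left mouse click.
; Front and Back overlap volumes track the player, and a relative-yaw check requires the Siren character to face the train.
; After a short delay, timelines move the mesh along local Y, forward from Back or backward from Front, with looping animations.
; An IsMoving flag blocks input during a move.
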(event `self.ReceiveBeginPlay`
  ;[1 1 1] whatMakesEverythingWork
  (`self.EnableInput` (`GameplayStatics.GetPlayerController` 0)))

(event `self.Back.OnComponentBeginOverlap`
  (params (OverlappedComponent :type "PrimitiveComponent Object Reference") (OtherActor :type "Actor Object Reference") (OtherComp :type "PrimitiveComponent Object Reference") (OtherBodyIndex :type Integer) (bFromSweep :type Boolean) (SweepResult :type "HitResult Structure (by ref)"))
  ;[1 0.8436 0] keys
  (if (== OtherActor (`GameplayStatics.GetPlayerCharacter` 0))
    (set `self.backVariable` true)))

(event `Key|LeftMouseButton` :consume false
  (params (Key :type "Key Structure"))
  (bind _returnvalue (`GameplayStatics.GetPlayerCharacter` 0))
  (bind _train (`self.Train`))
  (bind (_returnvalue_roll _returnvalue_pitch _returnvalue_yaw) (`KismetMathLibrary.BreakRotator` (`SceneComponent.K2_GetComponentRotation` (`self.Train`))))
  (bind (_returnvalue_roll_2 _returnvalue_pitch_2 _returnvalue_yaw_2) (`KismetMathLibrary.BreakRotator` (`SceneComponent.K2_GetComponentRotation` (`self.Train`))))
  (bind (_relativelocation_x _relativelocation_y) (`KismetMathLibrary.BreakVector` (`SceneComponent.RelativeLocation` (`self.Train`))))
  (bind _returnvalue_2 (< _relativelocation_y 156.0))
  ;[0.05642 0.3802 0.01054] doors
  (:`Pressed`
    (if (`self.frontVariable`)
      (if (not (`self.is moving`))
        (bind _asbp_third_person_character_matrioska_siren (cast `/Game/matrioska/BP_ThirdPersonCharacterMatrioskaSiren` _returnvalue))
        (bind (_returnvalue_roll_3 _returnvalue_pitch_3 _returnvalue_yaw_3) (`KismetMathLibrary.BreakRotator` (`SceneComponent.K2_GetComponentRotation` (`Actor.RootComponent` _asbp_third_person_character_matrioska_siren))))
        (bind _returnvalue_3 (- _returnvalue_yaw_3 _returnvalue_yaw))
        (if (and (> _returnvalue_3 -135.0) (< _returnvalue_3 -45.0))
          (set `self.is moving` true)
          (if (not _returnvalue_2)
            ;[1 0 0.3026] actions
            (`KismetSystemLibrary.Delay` 0.6)
            (bind (_direction _y) (`Timeline|reversed` :!via `ReverseFromEnd`)
              (:`Update`
                (`SceneComponent.K2_SetRelativeLocation` _train (`KismetMathLibrary.MakeVector` 0.0 _y) false false)
                (`/Engine/EditorBlueprintResources/StandardMacros.DoOnce` false
                  (:`Completed`
                    (`SkeletalMeshComponent.PlayAnimation` _train "/Game/matrioska/OtherElements/trainPuzzle/trainParts/bacwards.bacwards" true))))
              (:`Finished`
                (`SkeletalMeshComponent.Stop` _train)
                (set `self.is moving` false :!label _label))))))
      (elif (`self.backVariable`)
        (if (not (`self.is moving`))
          (bind _asbp_third_person_character_matrioska_siren_2 (cast `/Game/matrioska/BP_ThirdPersonCharacterMatrioskaSiren` _returnvalue))
          (bind (_returnvalue_roll_4 _returnvalue_pitch_4 _returnvalue_yaw_4) (`KismetMathLibrary.BreakRotator` (`SceneComponent.K2_GetComponentRotation` (`Actor.RootComponent` _asbp_third_person_character_matrioska_siren_2))))
          (bind _returnvalue_4 (- _returnvalue_yaw_4 _returnvalue_yaw_2))
          (if (and (> _returnvalue_4 45.0) (< _returnvalue_4 135.0))
            (set `self.is moving` true)
            (if _returnvalue_2
              (`KismetSystemLibrary.Delay` 0.6)
              (bind (_direction_2 _y_2) (`Timeline|advanced` :!via `PlayFromStart`)
                (:`Update`
                  (`SceneComponent.K2_SetRelativeLocation` _train (`KismetMathLibrary.MakeVector` 0.0 _y_2) false false)
                  (`/Engine/EditorBlueprintResources/StandardMacros.DoOnce` false
                    (:`Completed`
                      (`SkeletalMeshComponent.PlayAnimation` _train "/Game/matrioska/OtherElements/trainPuzzle/trainParts/forward.forward" true))))
                (:`Finished`
                  (`SkeletalMeshComponent.Stop` _train)
                  (goto _label))))))))))

(event `self.Back.OnComponentEndOverlap`
  (params (OverlappedComponent :type "PrimitiveComponent Object Reference") (OtherActor :type "Actor Object Reference") (OtherComp :type "PrimitiveComponent Object Reference") (OtherBodyIndex :type Integer))
  ;[1 0.8436 0] keys
  (if (== OtherActor (`GameplayStatics.GetPlayerCharacter` 0))
    (set `self.backVariable` false)))

(event `self.Front.OnComponentBeginOverlap`
  (params (OverlappedComponent :type "PrimitiveComponent Object Reference") (OtherActor :type "Actor Object Reference") (OtherComp :type "PrimitiveComponent Object Reference") (OtherBodyIndex :type Integer) (bFromSweep :type Boolean) (SweepResult :type "HitResult Structure (by ref)"))
  ;[1 0.8436 0] keys
  (if (== OtherActor (`GameplayStatics.GetPlayerCharacter` 0))
    (set `self.frontVariable` true)))

(event `self.Front.OnComponentEndOverlap`
  (params (OverlappedComponent :type "PrimitiveComponent Object Reference") (OtherActor :type "Actor Object Reference") (OtherComp :type "PrimitiveComponent Object Reference") (OtherBodyIndex :type Integer))
  ;[1 0.8436 0] keys
  (if (== OtherActor (`GameplayStatics.GetPlayerCharacter` 0))
    (set `self.frontVariable` false)))

(fn `UserConstructionScript`)